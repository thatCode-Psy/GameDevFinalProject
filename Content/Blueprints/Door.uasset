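; Door actor that toggles an animated skeletal mesh door open and closed.
; On BeginPlay it sets the DoorOpening flag on the mesh's OpenDoorBlueprint anim instance to false.
; InteractDoor flips that flag, and both Hit events and Box overlap begins call it, then print a debug "Hello".
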(event `self.ReceiveBeginPlay`
  (bind _asopen_door_blueprint (cast `/Game/Blueprints/OpenDoorBlueprint` (`SkeletalMeshComponent.GetAnimInstance` (`self.SkeletalMesh`))))
  (set `/Game/Blueprints/OpenDoorBlueprint.DoorOpening` false _asopen_door_blueprint))

(event `self.ReceiveTick`
  (params (DeltaSeconds :type "Float (single-precision)")))

(event `self.ReceiveHit`
  (params (MyComp :type "PrimitiveComponent Object Reference") (Other :type "Actor Object Reference") (OtherComp :type "PrimitiveComponent Object Reference") (bSelfMoved :type Boolean) (HitLocation :type "Vector Structure") (HitNormal :type "Vector Structure") (NormalImpulse :type "Vector Structure") (Hit :type "HitResult Structure (by ref)"))
  (`self.InteractDoor` :!label _label)
  (`KismetSystemLibrary.PrintString` "Hello"))

(event `self.Box.OnComponentBeginOverlap`
  (params (OverlappedComponent :type "PrimitiveComponent Object Reference") (OtherActor :type "Actor Object Reference") (OtherComp :type "PrimitiveComponent Object Reference") (OtherBodyIndex :type Integer) (bFromSweep :type Boolean) (SweepResult :type "HitResult Structure (by ref)"))
  (goto _label))

(fn `InteractDoor`
  (bind _asopen_door_blueprint (cast `/Game/Blueprints/OpenDoorBlueprint` (`SkeletalMeshComponent.GetAnimInstance` (`self.SkeletalMesh`))))
  (if (`/Game/Blueprints/OpenDoorBlueprint.DoorOpening` _asopen_door_blueprint)
    (set `/Game/Blueprints/OpenDoorBlueprint.DoorOpening` false _asopen_door_blueprint)
    (else
      (set `/Game/Blueprints/OpenDoorBlueprint.DoorOpening` true _asopen_door_blueprint))))

(fn `UserConstructionScript`)