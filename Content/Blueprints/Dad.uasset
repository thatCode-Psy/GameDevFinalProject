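; Dad character that seizes the player on contact and lifts them off the ground, with its mesh hidden at BeginPlay.
; Hitting the Player stops its movement, turns off its own gravity and physics interaction, sets Seizing on its animation Blueprint and clears the player's LookingAtFather flag.
; Tick uses the recorded grab time to lerp the player upward over a fixed duration, printing debug values.
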(event `self.ReceiveBeginPlay`
  (`SceneComponent.SetVisibility` (`self.Mesh`) false false)
  (set `self.StartGrabTime` -1.0))

(event `self.ReceiveHit`
  (params (MyComp :type "PrimitiveComponent Object Reference") (Other :type "Actor Object Reference") (OtherComp :type "PrimitiveComponent Object Reference") (bSelfMoved :type Boolean) (HitLocation :type "Vector Structure") (HitNormal :type "Vector Structure") (NormalImpulse :type "Vector Structure") (Hit :type "HitResult Structure (by ref)"))
  (bind _charactermovement (`self.CharacterMovement`))
  (bind _asplayer (cast `/Game/Blueprints/Player` Other))
  (`MovementComponent.StopMovementImmediately` (`self.CharacterMovement`))
  (bind _asdad_animation_blueprint (cast `/Game/Blueprints/DadAnimationBlueprint` (`SkeletalMeshComponent.GetAnimInstance` (`self.Mesh`))))
  (if (not (`/Game/Blueprints/DadAnimationBlueprint.Seizing` _asdad_animation_blueprint))
    (set `/Game/Blueprints/DadAnimationBlueprint.Seizing` true _asdad_animation_blueprint)
    (set `CharacterMovementComponent.GravityScale` 0.0 _charactermovement)
    (set `CharacterMovementComponent.bEnablePhysicsInteraction` false _charactermovement)
    (set `self.StartGrabTime` (`GameplayStatics.GetTimeSeconds`))
    (set `/Game/Blueprints/Player.LookingAtFather` false _asplayer)
    (set `self.OriginalPlayerLocation` (`self.K2_GetActorLocation` _asplayer))))

(event `self.ReceiveTick`
  (params (DeltaSeconds :type "Float (single-precision)"))
  (bind _originalplayerlocation (`self.OriginalPlayerLocation`))
  (bind _returnvalue (/ (- (`GameplayStatics.GetTimeSeconds`) (`self.StartGrabTime`)) 2.625))
  (bind _returnvalue_2 (`KismetMathLibrary.VLerp` _originalplayerlocation (+ _originalplayerlocation (0.0 0.0 48.0)) _returnvalue))
  (if (>= (`self.StartGrabTime`) 0.0)
    (if (< _returnvalue 1.0)
      (`self.K2_SetActorLocation` (stale `self.ReceiveHit` _asplayer) _returnvalue_2 false false)
      (`KismetSystemLibrary.PrintString` (`KismetStringLibrary.Concat_StrStr` (`KismetStringLibrary.Conv_VectorToString` _returnvalue_2) "float " (`KismetStringLibrary.Conv_DoubleToString` _returnvalue))))))

(fn `UserConstructionScript`)