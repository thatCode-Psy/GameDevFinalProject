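; WallManager is an actor that switches four referenced walls to an alert material when the level starts with a wall trigger flag set.
; On BeginPlay it casts the game instance to PTSDGameInstance and reads IsWallTrigger.
; If the flag is true, it applies AlertMaterial to the first material slot of each wall's static mesh.
; The check runs only once, with no overlap or tick logic.
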(event `self.ReceiveBeginPlay`
  (bind _alertmaterial (`self.AlertMaterial`))
  (bind _asptsdgame_instance (cast `/Game/Blueprints/PTSDGameInstance` (`GameplayStatics.GetGameInstance`)))
  (if (`/Game/Blueprints/PTSDGameInstance.IsWallTrigger` _asptsdgame_instance)
    (`PrimitiveComponent.SetMaterial` (`StaticMeshActor.StaticMeshComponent` (`self.Wall1`)) 0 _alertmaterial)
    (`PrimitiveComponent.SetMaterial` (`StaticMeshActor.StaticMeshComponent` (`self.Wall2`)) 0 _alertmaterial)
    (`PrimitiveComponent.SetMaterial` (`StaticMeshActor.StaticMeshComponent` (`self.Wall3`)) 0 _alertmaterial)
    (`PrimitiveComponent.SetMaterial` (`StaticMeshActor.StaticMeshComponent` (`self.Wall4`)) 0 _alertmaterial)))

(fn `UserConstructionScript`)