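; Car actor that holds path-following state for one of three predefined paths; the file contains no movement logic.
; The construction script gives the mesh a random Beetle color material and sets its tag to Problem.
; BeginPlay resets the current node index to zero.
; SetCurrentPathOfCar copies the path matching PathNumber into CurrentPath, but nothing in this file calls it.
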(event `self.ReceiveBeginPlay`
  (set `self.CurrentNode` 0))

(fn `SetCurrentPathOfCar`
  (switch `int` (`self.PathNumber`)
    (:`0`
      (set `self.CurrentPath` (`self.Path0`)))
    (:`1`
      (set `self.CurrentPath` (`self.Path1`)))
    (:`2`
      (set `self.CurrentPath` (`self.Path2`)))))

(fn `UserConstructionScript`
  (bind _beetlecarcolors (`self.BeetleCarColors`))
  (`PrimitiveComponent.SetMaterial` (`self.StaticMesh`) 0 (`|GetArrayItem` _beetlecarcolors (`KismetMathLibrary.RandomInteger` (`KismetArrayLibrary.Array_Length` _beetlecarcolors))))
  (set `self.Tag` (struct :`TagName` "Problem")))